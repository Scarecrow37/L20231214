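; BP_Rocket is a projectile actor that flies forward and explodes when it overlaps something.
; BeginPlay sets its lifespan, and Tick offsets it along its local X axis by Velocity scaled by delta time, with no projectile movement component driving it.
; Any overlap on the Box component spawns an explosion emitter and sound at the rocket's location, then destroys the actor without applying damage.
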(event OnComponentBeginOverlap(Box)
  (params (OverlappedComponent :type Primitive%20Component%20Object%20Reference) (OtherActor :type Actor%20Object%20Reference) (OtherComp :type Primitive%20Component%20Object%20Reference) (OtherBodyIndex :type Integer) (bFromSweep :type Boolean) (SweepResult :type Hit%20Result%20Structure%20%28by%20ref%29))
  (Effects|SpawnEmitteratLocation "/Game/StarterContent/Particles/P_Explosion.P_Explosion" (Transformation|GetActorLocation))
  (Audio|PlaySoundatLocation "/Game/StarterContent/Audio/Explosion01.Explosion01" (Transformation|GetActorLocation) "0, 0, 0" 1.0 1.0 0.0 0 0 0 0)
  (Actor|DestroyActor))

(event EventBeginPlay
  (Actor|SetLifeSpan (Variables|Life|GetLifespan)))

(event EventTick
  (params (DeltaSeconds :type Float%20%28single-precision%29))
  (Transformation|AddActorLocalOffset (Math|Vector|MakeVector (* DeltaSeconds (Variables|Movement|GetVelocity)) 0.0 0.0) false false))

(fn ConstructionScript)