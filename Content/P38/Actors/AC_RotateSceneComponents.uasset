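; Actor component that continuously spins a list of scene components by adding relative rotation to each one every tick.
; ClampAndLerpRotation clamps each axis of RotateValue to 0–1 and uses it as a lerp alpha between zero and Velocity scaled by world delta seconds.
; RotateValue thus acts as a per-axis weight, with negative inputs yielding no rotation, while Velocity sets a frame-rate-independent speed.
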(event EventTick
  (params (DeltaSeconds :type Float%20%28single-precision%29))
  (bind _outrotation (CallFunction|ClampandLerpRotation (Variables|Movement|GetRotateValue) 0.0 (* (Utilities|Time|GetWorldDeltaSeconds) (Variables|Movement|GetVelocity))))
  (Variables|Default|SetDeltaRotation _outrotation)
  (for _array_element (Variables|Target|GetSceneComponents)
    (Transformation|AddRelativeRotation _array_element (Variables|Default|GetDeltaRotation) false false)))

(fn ClampandLerpRotation
  (params (InRotation :type Rotator) (MinValue :type Float%20%28double-precision%29) (MaxValue :type Float%20%28double-precision%29))
  (Utilities|FlowControl|Sequence
    (:then_0
      (LocalVariables|SetRoll (.roll InRotation)))
    (:then_1
      (LocalVariables|SetPitch (.pitch InRotation)))
    (:then_2
      (LocalVariables|SetYaw (.yaw InRotation)))
    (:then_3
      (LocalVariables|SetMin MinValue))
    (:then_4
      (LocalVariables|SetMax MaxValue))
    (:then_5
      (return (Math|Rotator|MakeRotator (Math|Float|Lerp (LocalVariables|GetMin) (LocalVariables|GetMax) (Math|Float|Clamp(Float) (LocalVariables|GetRoll))) (Math|Float|Lerp (LocalVariables|GetMin) (LocalVariables|GetMax) (Math|Float|Clamp(Float) (LocalVariables|GetPitch))) (Math|Float|Lerp (LocalVariables|GetMin) (LocalVariables|GetMax) (Math|Float|Clamp(Float) (LocalVariables|GetYaw))))))))